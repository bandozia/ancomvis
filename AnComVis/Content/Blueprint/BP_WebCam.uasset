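; BP_WebCam shows a webcam feed on a mesh and marks detected face landmarks with debug spheres.
; At BeginPlay it applies a dynamic instance of M_WebCam to the viewer mesh.
; Each OnNextFrame event pushes VideoTexture into that material and draws short-lived red spheres at every landmark in DetectedFaces.
; The graph only consumes the video and detection data; it does not compute them.
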(event `self.ReceiveBeginPlay`
  (bind _returnvalue (`PrimitiveComponent.CreateDynamicMaterialInstance` (`self.ViwerStaticMesh`) 0 "/AnComVis/Material/M_WebCam.M_WebCam" "None"))
  (`PrimitiveComponent.SetMaterial` (`self.ViwerStaticMesh`) 0 _returnvalue)
  (set `self.DynamicMaterial` _returnvalue))

(event `self.OnNextFrame`
  (`MaterialInstanceDynamic.SetTextureParameterValue` (`self.DynamicMaterial`) "Texture" (`self.VideoTexture`))
  (for _array_element (`self.DetectedFaces`)
    (for _array_element_2 (`.LandMarks` (break `FaceDetected` _array_element))
      (`KismetSystemLibrary.DrawDebugSphere` (`KismetMathLibrary.MakeVector` (`KismetMathLibrary.BreakVector2D` _array_element_2) (`.Y` (`KismetMathLibrary.BreakVector2D` _array_element_2))) 1.0 6 (struct :`R` 0.817708 :`B` 0.075542 :`A` 1.0) 0.1 0.3))))

(fn `UserConstructionScript`)